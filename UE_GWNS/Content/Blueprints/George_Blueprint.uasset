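; George_Blueprint is a player-controlled side-scrolling character that runs along the world X axis and jumps.
; The MoveRight axis feeds movement input and sets the controller yaw to 0 or 180 according to its sign, turning the character to face its direction of travel.
; The Jump action triggers a jump, and BeginPlay turns on replication for the Sprite component.
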(event `self.ReceiveBeginPlay`
  ;[1 1 1] for multiplayer i guess
  (`ActorComponent.SetIsReplicated` (`self.Sprite`) true))

(event `self.ReceiveActorBeginOverlap`
  (params (OtherActor :type "Actor Object Reference")))

(event `InputAxis|MoveRight`
  (params (AxisValue :type "Float (single-precision)"))
  (`self.AddMovementInput` (1.0 0.0 0.0) AxisValue)
  (`/Engine/EditorBlueprintResources/StandardMacros.CompareFloat` AxisValue
    (:`>`
      (`Controller.SetControlRotation` (`self.GetController`) (`KismetMathLibrary.MakeRot` 0.0)))
    (:`<`
      (`Controller.SetControlRotation` (`self.GetController`) (`KismetMathLibrary.MakeRot` 0.0 180.0)))))

(event `self.ReceiveTick`
  (params (DeltaSeconds :type "Float (single-precision)")))

(event `InputAction|Jump`
  (:`Pressed`
    (`self.Jump`)))

(fn `UserConstructionScript`)